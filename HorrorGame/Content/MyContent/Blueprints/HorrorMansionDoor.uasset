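; Automatic door for a horror mansion that swings open when anything overlaps its trigger volume and closes when the overlap ends.
; A timeline's Driver value plus the actor yaw cached in the construction script sets the Door component's relative yaw.
; Overlap end reverses the timeline from its end, even if the door is only partly open.
; The construction script also prints the cached rotation.
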(event `self.TriggerVolume.OnComponentBeginOverlap`
  (params (OverlappedComponent :type "PrimitiveComponent Object Reference") (OtherActor :type "Actor Object Reference") (OtherComp :type "PrimitiveComponent Object Reference") (OtherBodyIndex :type Integer) (bFromSweep :type Boolean) (SweepResult :type "HitResult Structure (by ref)"))
  (bind (_initialrotator_roll _initialrotator_pitch _initialrotator_yaw) (`KismetMathLibrary.BreakRotator` (`self.InitialRotator`)))
  (bind (_direction _driver) (`Timeline|Timeline-Door Driver` :!label _label)
    (:`Update`
      (`SceneComponent.K2_SetRelativeRotation` (`self.Door`) (`KismetMathLibrary.MakeRotator` 0.0 0.0 (+ _driver _initialrotator_yaw)) false false))))

(event `self.TriggerVolume.OnComponentEndOverlap`
  (params (OverlappedComponent :type "PrimitiveComponent Object Reference") (OtherActor :type "Actor Object Reference") (OtherComp :type "PrimitiveComponent Object Reference") (OtherBodyIndex :type Integer))
  (goto _label :!via `ReverseFromEnd`))

(fn `UserConstructionScript`
  (locals (InitalRotator :type "Rotator Structure" :default (struct)))
  (bind _returnvalue (`self.K2_GetActorRotation`))
  (`self.K2_SetActorRotation` _returnvalue)
  (bind _output_get (set `self.InitialRotator` _returnvalue))
  (`KismetSystemLibrary.PrintString` (`KismetStringLibrary.Conv_RotatorToString` _output_get)))