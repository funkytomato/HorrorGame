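; Wood pickup for the horror game's inventory, which becomes collectable a few seconds after spawning.
; On box overlap it fills the first empty of five character item slots, destroys itself and plays a sound, or prints that the inventory is full.
; Each pickup increments the character's wood count; on reaching three it shows an objective-complete widget, sets the "Light the fire" objective and writes it to the save slot.
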(event `self.ReceiveBeginPlay`
  (`KismetSystemLibrary.Delay` 3.0)
  (set `self.CanPickup` true))

(event `self.Box.OnComponentBeginOverlap`
  (params (OverlappedComponent :type "PrimitiveComponent Object Reference") (OtherActor :type "Actor Object Reference") (OtherComp :type "PrimitiveComponent Object Reference") (OtherBodyIndex :type Integer) (bFromSweep :type Boolean) (SweepResult :type "HitResult Structure (by ref)"))
  (bind _saversubclass (`self.SaverSubClass`))
  ;[1 1 1] Store items in Inventory slots
  (if (`self.CanPickup`)
    (bind _ashorror_third_person_character (cast `/Game/MyContent/Blueprints/HorrorThirdPersonCharacter` (`GameplayStatics.GetPlayerCharacter` 0)))
    (if (== (`/Game/MyContent/Blueprints/HorrorThirdPersonCharacter.Slot1Item` _ashorror_third_person_character) 0)
      (set `/Game/MyContent/Blueprints/HorrorThirdPersonCharacter.Slot1Item` 1 _ashorror_third_person_character)
      (`self.K2_DestroyActor` :!label _label)
      (`GameplayStatics.PlaySoundAtLocation` "/Game/StarterContent/Audio/Explosion01.Explosion01" (`self.K2_GetActorLocation` _ashorror_third_person_character) (struct) 1.0 1.0 0.0 null null null)
      ;[1 1 1] Check if objective accomplished
      (bind _ashorror_third_person_character_2 (cast `/Game/MyContent/Blueprints/HorrorThirdPersonCharacter` (`GameplayStatics.GetPlayerCharacter` 0)))
      ;[1 1 1] Display Collected Wood Objective Completed
      (bind _output_get (set `/Game/MyContent/Blueprints/HorrorThirdPersonCharacter.NumberOfWoodPieces` (+ (`/Game/MyContent/Blueprints/HorrorThirdPersonCharacter.NumberOfWoodPieces` _ashorror_third_person_character_2) 1) _ashorror_third_person_character_2))
      (`KismetSystemLibrary.PrintString` (`KismetStringLibrary.Conv_IntToString` _output_get))
      (if (== _output_get 3)
        (bind _returnvalue (`|CreateWidget` "/Game/MyContent/Blueprints/ObjectiveComplete.ObjectiveComplete_C"))
        (`UserWidget.AddToViewport` _returnvalue 0)
        ;[1 1 1] Set Light Fire Objective
        (bind _ashorror_third_person_character_3 (cast `/Game/MyContent/Blueprints/HorrorThirdPersonCharacter` (`GameplayStatics.GetPlayerCharacter` 0)))
        (set `/Game/MyContent/Blueprints/HorrorThirdPersonCharacter.PlayerObjective` "Light the fire!!!" _ashorror_third_person_character_3)
        (bind _returnvalue_2 (`GameplayStatics.DoesSaveGameExist` "HorrorSaveSlot"))
        (if _returnvalue_2
          (bind _returnvalue_3 (`GameplayStatics.LoadGameFromSlot` "HorrorSaveSlot"))
          (bind _output_get_2 (set `self.SaverSubClass` _returnvalue_3))
          (bind _ashorror_save_game (cast `/Game/MyContent/Blueprints/HorrorSaveGame` _output_get_2))
          (set `/Game/MyContent/Blueprints/HorrorSaveGame.PlayerObjective` "Light the fire!!!" _ashorror_save_game)
          (bind _returnvalue_4 (`GameplayStatics.SaveGameToSlot` _saversubclass "HorrorSaveSlot"))
          (`KismetSystemLibrary.PrintString` (`KismetStringLibrary.Conv_BoolToString` _returnvalue_4))
          (else
            (bind _returnvalue_5 (`GameplayStatics.CreateSaveGameObject` "/Game/MyContent/Blueprints/HorrorSaveGame.HorrorSaveGame_C"))
            (bind _output_get_3 (set `self.SaverSubClass` _returnvalue_5))
            (bind _ashorror_save_game_2 (cast `/Game/MyContent/Blueprints/HorrorSaveGame` _output_get_3))
            (set `/Game/MyContent/Blueprints/HorrorSaveGame.PlayerObjective` "Light the fire!!!" _ashorror_save_game_2)
            (bind _returnvalue_6 (`GameplayStatics.SaveGameToSlot` _saversubclass "HorrorSaveSlot"))
            (`KismetSystemLibrary.PrintString` (`KismetStringLibrary.Conv_BoolToString` _returnvalue_6)))))
      (elif (== (`/Game/MyContent/Blueprints/HorrorThirdPersonCharacter.Slot2Item` _ashorror_third_person_character) 0)
        (set `/Game/MyContent/Blueprints/HorrorThirdPersonCharacter.Slot2Item` 1 _ashorror_third_person_character)
        (goto _label)
        (elif (== (`/Game/MyContent/Blueprints/HorrorThirdPersonCharacter.Slot3Item` _ashorror_third_person_character) 0)
          (set `/Game/MyContent/Blueprints/HorrorThirdPersonCharacter.Slot3Item` 1 _ashorror_third_person_character)
          (goto _label)
          (elif (== (`/Game/MyContent/Blueprints/HorrorThirdPersonCharacter.Slot4Item` _ashorror_third_person_character) 0)
            (set `/Game/MyContent/Blueprints/HorrorThirdPersonCharacter.Slot4Item` 1 _ashorror_third_person_character)
            (goto _label)
            (elif (== (`/Game/MyContent/Blueprints/HorrorThirdPersonCharacter.Slot5Item` _ashorror_third_person_character) 0)
              (set `/Game/MyContent/Blueprints/HorrorThirdPersonCharacter.Slot5Item` 1 _ashorror_third_person_character)
              (goto _label)
              (else
                (`KismetSystemLibrary.PrintString` "Inventory is full!")))))))))

(fn `UserConstructionScript`)