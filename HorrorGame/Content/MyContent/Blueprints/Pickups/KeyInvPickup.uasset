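; Key inventory pickup for the horror third-person character, which becomes collectable after a short delay from BeginPlay.
; Any overlap on its box casts the player character, without checking the overlapping actor, and fills the first empty of five inventory slots with the key's item ID.
; On success it destroys itself, sets HasKey and plays a sound at the player; otherwise it prints that the inventory is full.
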(event `self.ReceiveBeginPlay`
  (`KismetSystemLibrary.Delay` 3.0)
  (set `self.CanPickup` true))

(event `self.Box.OnComponentBeginOverlap`
  (params (OverlappedComponent :type "PrimitiveComponent Object Reference") (OtherActor :type "Actor Object Reference") (OtherComp :type "PrimitiveComponent Object Reference") (OtherBodyIndex :type Integer) (bFromSweep :type Boolean) (SweepResult :type "HitResult Structure (by ref)"))
  (if (`self.CanPickup`)
    (bind _ashorror_third_person_character (cast `/Game/MyContent/Blueprints/HorrorThirdPersonCharacter` (`GameplayStatics.GetPlayerCharacter` 0)))
    (if (== (`/Game/MyContent/Blueprints/HorrorThirdPersonCharacter.Slot1Item` _ashorror_third_person_character) 0)
      (set `/Game/MyContent/Blueprints/HorrorThirdPersonCharacter.Slot1Item` 2 _ashorror_third_person_character)
      (`self.K2_DestroyActor` :!label _label)
      (bind _ashorror_third_person_character_2 (cast `/Game/MyContent/Blueprints/HorrorThirdPersonCharacter` (`GameplayStatics.GetPlayerCharacter` 0)))
      (set `/Game/MyContent/Blueprints/HorrorThirdPersonCharacter.HasKey` true _ashorror_third_person_character_2)
      (`GameplayStatics.PlaySoundAtLocation` "/Game/StarterContent/Audio/Explosion01.Explosion01" (`self.K2_GetActorLocation` _ashorror_third_person_character) (struct) 1.0 1.0 0.0 null null null)
      (elif (== (`/Game/MyContent/Blueprints/HorrorThirdPersonCharacter.Slot2Item` _ashorror_third_person_character) 0)
        (set `/Game/MyContent/Blueprints/HorrorThirdPersonCharacter.Slot2Item` 2 _ashorror_third_person_character)
        (goto _label)
        (elif (== (`/Game/MyContent/Blueprints/HorrorThirdPersonCharacter.Slot3Item` _ashorror_third_person_character) 0)
          (set `/Game/MyContent/Blueprints/HorrorThirdPersonCharacter.Slot3Item` 2 _ashorror_third_person_character)
          (goto _label)
          (elif (== (`/Game/MyContent/Blueprints/HorrorThirdPersonCharacter.Slot4Item` _ashorror_third_person_character) 0)
            (set `/Game/MyContent/Blueprints/HorrorThirdPersonCharacter.Slot4Item` 2 _ashorror_third_person_character)
            (goto _label)
            (elif (== (`/Game/MyContent/Blueprints/HorrorThirdPersonCharacter.Slot5Item` _ashorror_third_person_character) 0)
              (set `/Game/MyContent/Blueprints/HorrorThirdPersonCharacter.Slot5Item` 2 _ashorror_third_person_character)
              (goto _label)
              (else
                (`KismetSystemLibrary.PrintString` "Inventory is full!")))))))))

(fn `UserConstructionScript`)