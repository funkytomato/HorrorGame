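; Objective trigger actor that sets the player's objective to "Find the key" when the horror third-person character overlaps it.
; It writes the objective on the character, then loads the existing horror save game or creates a new one, stores the objective there and saves it to the slot.
; Debug prints report the load or create branch and the save result.
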(event `self.ReceiveActorBeginOverlap`
  (params (OtherActor :type "Actor Object Reference"))
  (bind _saversubclass (`self.SaverSubClass`))
  (bind _ashorror_third_person_character (cast `/Game/MyContent/Blueprints/HorrorThirdPersonCharacter` OtherActor))
  ;[1 1 1] Save Player Objective
  (set `/Game/MyContent/Blueprints/HorrorThirdPersonCharacter.PlayerObjective` "Find the key" _ashorror_third_person_character)
  (bind _returnvalue (`GameplayStatics.DoesSaveGameExist` "HorrorSaveSlot"))
  (if _returnvalue
    (`KismetSystemLibrary.PrintString` "Loading SaveGame")
    (bind _returnvalue_2 (`GameplayStatics.LoadGameFromSlot` "HorrorSaveSlot"))
    (bind _output_get (set `self.SaverSubClass` _returnvalue_2))
    (bind _ashorror_save_game (cast `/Game/MyContent/Blueprints/HorrorSaveGame` _output_get))
    (set `/Game/MyContent/Blueprints/HorrorSaveGame.PlayerObjective` "Find the key" _ashorror_save_game)
    (bind _returnvalue_3 (`GameplayStatics.SaveGameToSlot` _saversubclass "HorrorSaveSlot"))
    (`KismetSystemLibrary.PrintString` (`KismetStringLibrary.Conv_BoolToString` _returnvalue_3))
    (else
      (`KismetSystemLibrary.PrintString` "Creating SaveGame")
      (bind _returnvalue_4 (`GameplayStatics.CreateSaveGameObject` "/Game/MyContent/Blueprints/HorrorSaveGame.HorrorSaveGame_C"))
      (bind _output_get_2 (set `self.SaverSubClass` _returnvalue_4))
      (bind _ashorror_save_game_2 (cast `/Game/MyContent/Blueprints/HorrorSaveGame` _output_get_2))
      (set `/Game/MyContent/Blueprints/HorrorSaveGame.PlayerObjective` "Find the key" _ashorror_save_game_2)
      (bind _returnvalue_5 (`GameplayStatics.SaveGameToSlot` _saversubclass "HorrorSaveSlot"))
      (`KismetSystemLibrary.PrintString` (`KismetStringLibrary.Conv_BoolToString` _returnvalue_5)))))

(fn `UserConstructionScript`)