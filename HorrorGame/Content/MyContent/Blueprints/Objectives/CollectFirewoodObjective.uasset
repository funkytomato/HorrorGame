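; Trigger actor that sets the horror player's current objective to "Collect Firewood" and persists it to the save game.
; On overlap by a HorrorThirdPersonCharacter, it writes the objective to the character, then loads the existing HorrorSaveSlot save or creates a new HorrorSaveGame.
; It stores the objective in that save object, saves it back to the slot and prints the save result.
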(event `self.ReceiveActorBeginOverlap`
  (params (OtherActor :type "Actor Object Reference"))
  (bind _saversubclass (`self.SaverSubClass`))
  ;[1 1 1] Save Player Objective
  (bind _ashorror_third_person_character (cast `/Game/MyContent/Blueprints/HorrorThirdPersonCharacter` OtherActor))
  (set `/Game/MyContent/Blueprints/HorrorThirdPersonCharacter.PlayerObjective` "Collect Firewood" _ashorror_third_person_character)
  (bind _returnvalue (`GameplayStatics.DoesSaveGameExist` "HorrorSaveSlot"))
  (if _returnvalue
    (bind _returnvalue_2 (`GameplayStatics.LoadGameFromSlot` "HorrorSaveSlot"))
    (bind _output_get (set `self.SaverSubClass` _returnvalue_2))
    (bind _ashorror_save_game (cast `/Game/MyContent/Blueprints/HorrorSaveGame` _output_get))
    (set `/Game/MyContent/Blueprints/HorrorSaveGame.PlayerObjective` "Collect Firewood" _ashorror_save_game)
    (bind _returnvalue_3 (`GameplayStatics.SaveGameToSlot` _saversubclass "HorrorSaveSlot"))
    (`KismetSystemLibrary.PrintString` (`KismetStringLibrary.Conv_BoolToString` _returnvalue_3))
    (else
      (bind _returnvalue_4 (`GameplayStatics.CreateSaveGameObject` "/Game/MyContent/Blueprints/HorrorSaveGame.HorrorSaveGame_C"))
      (bind _output_get_2 (set `self.SaverSubClass` _returnvalue_4))
      (bind _ashorror_save_game_2 (cast `/Game/MyContent/Blueprints/HorrorSaveGame` _output_get_2))
      (set `/Game/MyContent/Blueprints/HorrorSaveGame.PlayerObjective` "Collect Firewood" _ashorror_save_game_2)
      (bind _returnvalue_5 (`GameplayStatics.SaveGameToSlot` _saversubclass "HorrorSaveSlot"))
      (`KismetSystemLibrary.PrintString` (`KismetStringLibrary.Conv_BoolToString` _returnvalue_5)))))

(fn `UserConstructionScript`)